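; Stage camera rail actor that tracks a pawn along a spline while the pawn overlaps it.
; Overlap begin and end set or clear the follow target, toggle Tick and register or unregister the spline with that player's StagePlayerCameraManager.
; Each tick eases the camera toward the spline point closest to the target, plus an offset rotated to the spline direction, and smoothly turns it to face the target.
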(event Collision|EventActorBeginOverlap
  (params (OtherActor :type Actor%20Object%20Reference))
  (bind _aspawn (Utilities|Casting|CastToPawn OtherActor))
  (Public|SetTarget _aspawn))

(event EventTick
  (params (DeltaSeconds :type Float%20%28single-precision%29))
  (Private|UpdatefromTarget DeltaSeconds))

(event Collision|EventActorEndOverlap
  (params (OtherActor :type Actor%20Object%20Reference))
  (if (== OtherActor (Variables|Default|GetFollowTarget))
    (Public|SetTarget)))

(fn ConstructionScript)

(fn SetTarget
  (params (InTarget :type Pawn%20Object%20Reference))
  (if (!= InTarget (Variables|Default|GetFollowTarget))
    (Utilities|FlowControl|Sequence
      (:then_0
        (bind _cameramanager (Private|GetCameraManager (Variables|Default|GetFollowTarget)))
        (Utilities|IsValid _cameramanager
          (:Is%20Valid
            (Default|RemoveCameraSpline _cameramanager self))))
      (:then_1
        (bind _output_get (Variables|Default|SetFollowTarget InTarget))
        (Utilities|IsValid _output_get
          (:Is%20Valid
            (Actor|Tick|SetActorTickEnabled true)
            (bind _cameramanager_2 (Private|GetCameraManager (Variables|Default|GetFollowTarget)))
            (Utilities|IsValid _cameramanager_2
              (:Is%20Valid
                (Default|AddCameraSpline _cameramanager_2 self))))
          (:Is%20Not%20Valid
            (Actor|Tick|SetActorTickEnabled false)))))))

(fn UpdatefromTarget
  (params (DeltaTime :type Float%20%28single-precision%29))
  (bind _returnvalue (Math|Vector|MakeVector 0.0 0.0 1.0))
  (bind _offset (Variables|Default|GetOffset))
  (bind _spline (Variables|Default|GetSpline))
  (bind _followtarget (Variables|Default|GetFollowTarget))
  (bind _camera (Variables|Default|GetCamera))
  (bind _returnvalue_2 (Transformation|GetActorLocation _followtarget))
  (bind _returnvalue_3 (Spline|FindLocationClosesttoWorldLocation _spline _returnvalue_2 "World"))
  (bind _returnvalue_4 (Spline|FindDirectionClosesttoWorldLocation _spline _returnvalue_2 "World"))
  (bind _returnvalue_5 (Class|KismetMathLibrary|MakeRotfromYZ _returnvalue_4 _returnvalue))
  (bind _returnvalue_6 (Math|Vector|RotateVector _offset _returnvalue_5))
  (bind _returnvalue_7 (+ _returnvalue_3 _returnvalue_6))
  (Utilities|IsValid _followtarget
    (:Is%20Valid
      (Transformation|SetWorldLocationAndRotation (Variables|Default|GetCamera) (Math|Interpolation|VInterpTo (Transformation|GetWorldLocation _camera) _returnvalue_7 DeltaTime 5.0) (Math|Interpolation|RInterpTo (Transformation|GetWorldRotation _camera) (Math|Rotator|FindLookatRotation _returnvalue_7 _returnvalue_2) DeltaTime 1e+01) false false))))

(fn GetCameraManager
  (params (Pawn :type Pawn%20Object%20Reference))
  (Utilities|IsValid Pawn
    (:Is%20Valid
      (bind _asplayer_controller (Utilities|Casting|CastToPlayerController (Pawn|GetController Pawn))
        (:then
          (bind _asstage_player_camera_manager (Utilities|Casting|CastToStagePlayerCameraManager (Variables|/Script/Engine.PlayerController|GetPlayerCameraManager _asplayer_controller))
            (:then
              (return _asstage_player_camera_manager))
            (:CastFailed
              _)))
        (:CastFailed
          _)))
    (:Is%20Not%20Valid
      _))
  (return 0))