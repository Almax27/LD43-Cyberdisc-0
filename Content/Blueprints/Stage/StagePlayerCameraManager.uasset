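; Player camera manager for stages that tracks registered camera splines and switches the player's view between them.
; The first spline added becomes active, and later additions are only stored, with duplicates printing an error.
; Removing a spline activates the last one remaining, while an empty list leaves the current target in place.
; Changing the active spline blends the owning controller's view target with an eased, outgoing-locked transition.
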(event EventBeginPlay)

(event Collision|EventActorBeginOverlap
  (params (OtherActor :type Actor%20Object%20Reference)))

(event EventTick
  (params (DeltaSeconds :type Float%20%28single-precision%29)))

(fn ConstructionScript)

(fn AddCameraSpline
  (params (CameraSpline :type Stage%20Camera%20Spline%20Object%20Reference))
  (bind _camerasplines (Variables|Default|GetCameraSplines))
  (if (not (Utilities|Array|ContainsItem _camerasplines CameraSpline))
    (bind _returnvalue (Utilities|Array|Add _camerasplines CameraSpline))
    (if (== _returnvalue 0)
      (CallFunction|SetActiveCameraSpline CameraSpline))
    (else
      (Development|PrintString "CameraSpline added twice!!!" true true "(R=1.000000,G=0.000000,B=0.000000,A=1.000000)"))))

(fn RemoveCameraSpline
  (params (CameraSpline :type Stage%20Camera%20Spline%20Object%20Reference))
  (bind _camerasplines (Variables|Default|GetCameraSplines))
  (bind _returnvalue (Utilities|Array|Length _camerasplines))
  (bind _returnvalue_2 (- _returnvalue 1))
  (bind _returnvalue_3 (Utilities|Array|RemoveItem (Variables|Default|GetCameraSplines) CameraSpline))
  (if _returnvalue_3
    (if (Utilities|Array|IsValidIndex _camerasplines _returnvalue_2)
      (CallFunction|SetActiveCameraSpline (Utilities|Array|Get(acopy) _camerasplines _returnvalue_2)))))

(fn SetActiveCameraSpline
  (params (CameraSpline :type Stage%20Camera%20Spline%20Object%20Reference))
  (bind _returnvalue (Game|Player|GetOwningPlayerController))
  (if (!= CameraSpline (Variables|Default|GetActiveCameraSpline))
    (bind _output_get (Variables|Default|SetActiveCameraSpline CameraSpline))
    (Utilities|IsValid _returnvalue
      (:Is%20Valid
        (Game|Player|SetViewTargetwithBlend _returnvalue _output_get 1.0 "VTBlend_EaseInOut" 2.0 true)))))