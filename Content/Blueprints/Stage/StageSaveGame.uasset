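; StageSaveGame is a save game object that records the checkpoints reached in a stage and the most recent new one.
; ProcessCheckpoint adds an unseen checkpoint, saves the object to its slot and returns whether it was new.
; The OnCheckpointReached event makes the same update without saving.
; Save writes the object itself to the stored slot name and user index.
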(event Custom|OnCheckpointReached
  (params (Checkpoint :type Checkpoint%20Object%20Reference))
  (bind _checkpointsreached (Variables|SaveData|GetCheckpointsReached))
  (if (not (Utilities|Array|ContainsItem _checkpointsreached Checkpoint))
    (Utilities|Array|AddUnique _checkpointsreached Checkpoint)
    (Variables|SaveData|SetLastCheckPoint Checkpoint)))

(fn Save
  (SaveGame|SaveGametoSlot self (Variables|SaveInfo|GetSlotName) (Variables|SaveInfo|GetUserIndex)))

(fn ProcessCheckpoint
  (params (Checkpoint :type Checkpoint%20Object%20Reference))
  (bind _checkpointsreached (Variables|SaveData|GetCheckpointsReached))
  (if (Utilities|Array|ContainsItem _checkpointsreached Checkpoint)
    (return false)
    (else
      (Utilities|Array|AddUnique _checkpointsreached Checkpoint)
      (Variables|SaveData|SetLastCheckPoint Checkpoint)
      (CallFunction|Save)
      (return true))))