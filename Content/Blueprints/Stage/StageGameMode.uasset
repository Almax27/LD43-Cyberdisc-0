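; Stage game mode that persists progress in a StageSaveGame and picks the player start from the saved checkpoint name.
; GetSaveGame lazily caches the "StageSave" slot, creating and saving a new object if loading fails.
; ChoosePlayerStart compares Checkpoint actors with the saved name, but returns empty at the first mismatch, so only the first actor is effectively checked.
; The save is written back when the game mode is destroyed.
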(event EventDestroyed
  (bind _newparam (CallFunction|GetSaveGame))
  (Utilities|IsValid _newparam
    (:Is%20Valid
      (SaveGame|SaveGametoSlot _newparam (Variables|/Game/Blueprints/Stage/StageSaveGame.StageSaveGame_C|GetSlotName _newparam) (Variables|/Game/Blueprints/Stage/StageSaveGame.StageSaveGame_C|GetUserIndex _newparam)))))

(fn ConstructionScript)

(fn ChoosePlayerStart
  (params (Player :type Controller%20Object%20Reference))
  (bind _newparam (CallFunction|GetSaveGame))
  (Utilities|IsValid _newparam
    (:Is%20Valid
      (bind _outactors (Actor|GetAllActorsOfClass "/Game/Blueprints/Stage/Progression/Checkpoint.Checkpoint_C"))
      (for _array_element _outactors
        (if (Utilities|Name|Equal(Name) (Variables|/Game/Blueprints/Stage/Progression/Checkpoint.Checkpoint_C|GetCheckpointName _array_element) (Variables|/Game/Blueprints/Stage/StageSaveGame.StageSaveGame_C|GetCheckPointName _newparam))
          (return _array_element)
          (else
            (return 0)))))
    (:Is%20Not%20Valid
      _))
  (return 0))

(fn GetSaveGame
  (Utilities|FlowControl|Sequence
    (:then_0
      (Utilities|IsValid (Variables|Default|GetSaveGameInstance)
        (:Is%20Not%20Valid
          (bind _returnvalue (SaveGame|LoadGamefromSlot "StageSave"))
          (bind _asstage_save_game (Utilities|Casting|CastToStageSaveGame _returnvalue)
            (:then
              (Variables|Default|SetSaveGameInstance _asstage_save_game))
            (:CastFailed
              (bind _returnvalue_2 (SaveGame|CreateSaveGameObject "/Game/Blueprints/Stage/StageSaveGame.StageSaveGame_C"))
              (Utilities|IsValid _returnvalue_2
                (:Is%20Valid
                  (bind _output_get (Variables|Default|SetSaveGameInstance _returnvalue_2))
                  (SaveGame|SaveGametoSlot _output_get (Variables|/Game/Blueprints/Stage/StageSaveGame.StageSaveGame_C|GetSlotName _returnvalue_2) (Variables|/Game/Blueprints/Stage/StageSaveGame.StageSaveGame_C|GetUserIndex _returnvalue_2)))
                (:Is%20Not%20Valid
                  (Development|PrintString "Failed to create save" true true "(R=1.000000,G=0.000000,B=0.089263,A=1.000000)"))))))))
    (:then_1
      (return (Variables|Default|GetSaveGameInstance)))))